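; BP_Arrow_R is a vector visualizer that places red, green and blue arrowheads according to X, Y and Z length values.
; Each length is multiplied by 100 and set as its arrowhead's relative Z location.
; EditorTick and Tick share this update, so it runs in editor and game.
; The construction script also adds a child actor component, with no further setup shown.
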(event `/Game/CK_GGE/VectorVisualize/BPI_EditorTick.EditorTick`
  (`SceneComponent.K2_SetRelativeLocation` (`self.BP_Arrow_R_Arrow_Head`) (`KismetMathLibrary.MakeVector` 0.0 0.0 (* (`self.VectorLengthX`) 100.0)) false false :!label _label)
  (`SceneComponent.K2_SetRelativeLocation` (`self.BP_Arrow_G_Arrow_Head`) (`KismetMathLibrary.MakeVector` 0.0 0.0 (* (`self.VectorLengthY`) 100.0)) false false)
  (`SceneComponent.K2_SetRelativeLocation` (`self.BP_Arrow_B_Arrow_Head`) (`KismetMathLibrary.MakeVector` 0.0 0.0 (* (`self.VectorLengthZ`) 100.0)) false false))

(event `self.ReceiveTick`
  (params (DeltaSeconds :type "Float (single-precision)"))
  (goto _label))

(fn `UserConstructionScript`
  (`AddComponent|NODE_AddChildActorComponent-0`))