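; Actor that visualizes X, Y and Z vector lengths as three arrows (R, G, B), each built from a head and a shaft.
; Each length variable stretches its shaft along local Z and moves the head along that axis at 100 units per unit of length.
; EditorTick and Tick share this update, so the arrows follow the values both in the editor and at runtime.
; The construction script also adds a child actor component.
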(event `/Game/CK_GGE/EditorTick/BPI_EditorTick.EditorTick`
  (bind _vectorlengthx (`self.VectorLengthX`))
  (bind _vectorlengthy (`self.VectorLengthY`))
  (bind _vectorlengthz (`self.VectorLengthZ`))
  (`SceneComponent.K2_SetRelativeLocation` (`self.BP_Arrow_R_Head`) (`KismetMathLibrary.MakeVector` 0.0 0.0 (* _vectorlengthx 100.0)) false false :!label _label)
  (`SceneComponent.SetRelativeScale3D` (`self.BP_Arrow_R_Shaft`) (`KismetMathLibrary.MakeVector` 1.0 1.0 _vectorlengthx))
  (`SceneComponent.K2_SetRelativeLocation` (`self.BP_Arrow_G_Head`) (`KismetMathLibrary.MakeVector` 0.0 0.0 (* _vectorlengthy 100.0)) false false)
  (`SceneComponent.SetRelativeScale3D` (`self.BP_Arrow_G_Shaft`) (`KismetMathLibrary.MakeVector` 1.0 1.0 _vectorlengthy))
  (`SceneComponent.K2_SetRelativeLocation` (`self.BP_Arrow_B_Head`) (`KismetMathLibrary.MakeVector` 0.0 0.0 (* _vectorlengthz 100.0)) false false)
  (`SceneComponent.SetRelativeScale3D` (`self.BP_Arrow_B_Shaft`) (`KismetMathLibrary.MakeVector` 1.0 1.0 _vectorlengthz)))

(event `self.ReceiveTick`
  (params (DeltaSeconds :type "Float (single-precision)"))
  (goto _label))

(fn `UserConstructionScript`
  (`AddComponent|NODE_AddChildActorComponent-0`))