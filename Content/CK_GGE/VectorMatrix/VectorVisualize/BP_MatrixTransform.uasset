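; BP_MatrixTransform visualizes a basis-vector (matrix) transform on a toad mesh and a 2x2m cage mesh.
; Construction creates dynamic material instances for both meshes and adds a child actor component for editor ticking.
; On construction and each EditorTick, it feeds ArrowVectorActor's three arrowhead offsets from the shared root, scaled by 0.01, into the materials' BasisX, BasisY and BasisZ parameters, updating the view in editor.
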(event `/Game/CK_GGE/EditorTick/BPI_EditorTick.EditorTick`
  (`self.SetDynamicMaterials`))

(event `SetDynamicMaterials`
  (bind _arrowvectoractor (`self.ArrowVectorActor`))
  (bind _returnvalue (`SceneComponent.K2_GetComponentLocation` (`/Game/CK_GGE/VectorMatrix/VectorVisualize/BP_ArrowVector_XYZ.SharedRoot` _arrowvectoractor)))
  (bind _returnvalue_2 (`KismetMathLibrary.Conv_VectorToLinearColor` (* (- (`SceneComponent.K2_GetComponentLocation` (`/Game/CK_GGE/VectorMatrix/VectorVisualize/BP_ArrowVector_XYZ.BP_Arrow_G_Head` _arrowvectoractor)) _returnvalue) (0.01 0.01 0.01))))
  (bind _returnvalue_3 (`KismetMathLibrary.Conv_VectorToLinearColor` (* (- (`SceneComponent.K2_GetComponentLocation` (`/Game/CK_GGE/VectorMatrix/VectorVisualize/BP_ArrowVector_XYZ.BP_Arrow_B_Head` _arrowvectoractor)) _returnvalue) (0.01 0.01 0.01))))
  (bind _returnvalue_4 (`KismetMathLibrary.Conv_VectorToLinearColor` (* (- (`SceneComponent.K2_GetComponentLocation` (`/Game/CK_GGE/VectorMatrix/VectorVisualize/BP_ArrowVector_XYZ.BP_Arrow_R_Head` _arrowvectoractor)) _returnvalue) (0.01 0.01 0.01))))
  (for _array_element (`self.DynamicMaterialsA`)
    (`MaterialInstanceDynamic.SetVectorParameterValue` _array_element "BasisX" _returnvalue_4)
    (`MaterialInstanceDynamic.SetVectorParameterValue` _array_element "BasisY" _returnvalue_2)
    (`MaterialInstanceDynamic.SetVectorParameterValue` _array_element "BasisZ" _returnvalue_3)
    (for _array_element_2 (`self.DynamicMaterialsB`)
      (`MaterialInstanceDynamic.SetVectorParameterValue` _array_element_2 "BasisX" _returnvalue_4)
      (`MaterialInstanceDynamic.SetVectorParameterValue` _array_element_2 "BasisY" _returnvalue_2)
      (`MaterialInstanceDynamic.SetVectorParameterValue` _array_element_2 "BasisZ" _returnvalue_3))))

(fn `UserConstructionScript`
  (bind _2x2mcage (`self.2x2mCage`))
  (bind _jadetoad_5x (`self.JadeToad_5x`))
  (`AddComponent|NODE_AddChildActorComponent-0`) ; Editor Tick 컴포넌트 부착
  (for (_array_element _array_index) (`MeshComponent.GetMaterials` _jadetoad_5x)
    (bind _returnvalue (`PrimitiveComponent.CreateDynamicMaterialInstance` _jadetoad_5x _array_index _array_element "None"))
    (`KismetArrayLibrary.Array_Set` (`self.DynamicMaterialsA`) _array_index _returnvalue true)
    (for (_array_element_2 _array_index_2) (`MeshComponent.GetMaterials` _2x2mcage)
      (bind _returnvalue_2 (`PrimitiveComponent.CreateDynamicMaterialInstance` _2x2mcage _array_index_2 _array_element_2 "None"))
      (`KismetArrayLibrary.Array_Set` (`self.DynamicMaterialsB`) _array_index_2 _returnvalue_2 true))
    (`self.SetDynamicMaterials`)))