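; BP_TrigonometricRotate is an Actor Blueprint that demonstrates 2D rotation with trigonometry and matrices in the construction script.
; It places AngleSphere on a 100-unit circle in the XY plane using the cosine and sine of Angle.
; The same values, stored in AngleResult, build a Z-axis rotation matrix that transforms DefaultPos to position DefaultSphere.
; The event graph contains only empty default events.
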(fn `UserConstructionScript`
  (bind _angle (`self.Angle`))
  (bind _x (.x (`self.AngleResult`)))
  (bind _y (.y (`self.AngleResult`)))
  (bind _returnvalue (`KismetMathLibrary.MakeVector` (* (`KismetMathLibrary.DegCos` _angle) 1.0) (* (`KismetMathLibrary.DegSin` _angle) 1.0)))
  (`SceneComponent.K2_SetRelativeLocation` (`self.AngleSphere`) (* _returnvalue (100.0 100.0 100.0)) false false)
  (set `self.AngleResult` _returnvalue)
  (`SceneComponent.K2_SetRelativeLocation` (`self.DefaultSphere`) (`KismetMathLibrary.Conv_Vector4ToVector` (`KismetMathLibrary.Matrix_TransformVector` (make `Matrix` (make `Plane` 0.0 _x _y) (make `Plane` 0.0 (* _y -1.0) _x) (make `Plane` 0.0 0.0 0.0 1.0) (make `Plane` 1.0)) (`self.DefaultPos`))) false false))