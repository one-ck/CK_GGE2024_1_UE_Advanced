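; Actor Blueprint that recolors the JadeToad5x mesh at runtime through dynamic material instances.
; On BeginPlay it creates a dynamic instance for each of the mesh's material slots and caches them by index in DynamicMaterials.
; It then calls the SetDynamicMaterials event, which writes DynamicColor to the BaseColor vector parameter of every cached instance.
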(event `self.ReceiveBeginPlay`
  (bind _jadetoad_5x (`self.JadeToad_5x`))
  (for (_array_element _array_index) (`MeshComponent.GetMaterials` _jadetoad_5x)
    (bind _returnvalue (`PrimitiveComponent.CreateDynamicMaterialInstance` _jadetoad_5x _array_index _array_element "None"))
    (`KismetArrayLibrary.Array_Set` (`self.DynamicMaterials`) _array_index _returnvalue true))
  (`self.SetDynamicMaterials`))

(event `SetDynamicMaterials`
  (for _array_element (`self.DynamicMaterials`)
    (`MaterialInstanceDynamic.SetVectorParameterValue` _array_element "BaseColor" (`self.DynamicColor`))))

(fn `UserConstructionScript`)