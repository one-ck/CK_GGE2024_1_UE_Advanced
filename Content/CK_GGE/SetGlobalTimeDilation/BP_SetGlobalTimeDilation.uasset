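; Debug actor that controls game speed from the keyboard through global time dilation.
; BeginPlay enables its input only in builds not packaged for distribution, as a safety guard.
; P toggles pause by setting dilation to zero and restoring the stored TimeScale.
; Equals and Hyphen double or halve TimeScale and Backspace resets it, each also clearing the paused state.
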(event `self.ReceiveBeginPlay`
  (bind _returnvalue (`GameplayStatics.GetPlayerController` 0))
  ;[0.1545 0.1545 0.1545 1 14] 안전을 위해 배포용 빌드가 아닌 경우에만 키보드 입력을 받는다
  (if (`KismetSystemLibrary.IsPackagedForDistribution`)
    (`self.DisableInput` _returnvalue)
    (else
      (`self.EnableInput` _returnvalue))))

(event `Key|P`
  (params (Key :type "Key Structure"))
  (:`Pressed`
    (if (`self.Paused`)
      (`GameplayStatics.SetGlobalTimeDilation` (`self.TimeScale`)) ; Pause Off
      (set `self.Paused` false)
      (else
        (`GameplayStatics.SetGlobalTimeDilation` 0.0) ; Pause On
        (set `self.Paused` true)))))

(event `Key|Equals`
  (params (Key :type "Key Structure"))
  (:`Pressed`
    (bind _output_get (set `self.TimeScale` (* (`self.TimeScale`) 2.0)))
    (`GameplayStatics.SetGlobalTimeDilation` _output_get)
    (set `self.Paused` false) ; 무조건 Pause 해제
  ))

(event `Key|Hyphen`
  (params (Key :type "Key Structure"))
  (:`Pressed`
    (bind _output_get (set `self.TimeScale` (* (`self.TimeScale`) 0.5)))
    (`GameplayStatics.SetGlobalTimeDilation` _output_get)
    (set `self.Paused` false) ; 무조건 Pause 해제
  ))

(event `Key|BackSpace`
  (params (Key :type "Key Structure"))
  (:`Pressed`
    (set `self.TimeScale` 1.0)
    (set `self.Paused` false)
    (`GameplayStatics.SetGlobalTimeDilation` 1.0)))

(fn `UserConstructionScript`)